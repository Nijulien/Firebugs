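; BP_BigReactor is a reactor actor that adds to the player's count of activated energy when it is switched on.
; BeginPlay sets its point light to the off-state radius and intensity, and this file never changes the light afterward.
; Tick polls IsON, which is not set here, and uses a DoOnce to increment EnergyActivate on the BP_FirstPersonCharacter pawn a single time.
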(event EventTick
  (params (DeltaSeconds :type Float%20%28single-precision%29))
  (if (Variables|Default|GetIsON)
    (Utilities|FlowControl|DoOnce false
      (:Completed
        (bind _asbp_first_person_character (Utilities|Casting|CastToBP_FirstPersonCharacter (Game|Player|GetPlayerPawn 0)))
        (bind _result (Math|Integer|IncrementInt (Variables|/Game/FirstPerson/Blueprints/BP_FirstPersonCharacter.BP_FirstPersonCharacter_C|GetEnergyActivate _asbp_first_person_character))
          (:%20%20
            (Variables|/Game/FirstPerson/Blueprints/BP_FirstPersonCharacter.BP_FirstPersonCharacter_C|SetEnergyActivate _asbp_first_person_character _result)))))))

(event EventBeginPlay
  (Rendering|Lighting|SetAttenuationRadius (Variables|Default|GetPointLight) (Variables|Default|GetOffLightRadius))
  (Rendering|Components|Light|SetIntensity (Variables|Default|GetPointLight) (Variables|Default|GetOffLightIntensity)))

(fn ConstructionScript)