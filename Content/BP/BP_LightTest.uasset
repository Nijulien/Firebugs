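; Test light actor that grows and shrinks its point light as IsON switches, starting from the off radius and intensity.
; While on, Tick moves the player character's FireFlies component to the light.
; Two DoOnce gates run the on and off timelines once per switch, each timeline re-arming the other gate when finished.
; The timelines animate attenuation radius, while intensity snaps to its on or off value.
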(event EventTick
  (params (DeltaSeconds :type Float%20%28single-precision%29))
  (bind _pointlight (Variables|Default|GetPointLight))
  (bind _pointlight_2 (Variables|Default|GetPointLight))
  (if (Variables|Default|GetIsON)
    (bind _asbp_first_person_character (Utilities|Casting|CastToBP_FirstPersonCharacter (Game|Player|GetPlayerPawn 0)))
    (Transformation|SetWorldLocation (Variables|/Game/FirstPerson/Blueprints/BP_FirstPersonCharacter.BP_FirstPersonCharacter_C|GetFireFlies _asbp_first_person_character) (Transformation|GetWorldLocation (Variables|Default|GetPointLight)) false false)
    (Utilities|FlowControl|DoOnce false :!label _label
      (:Completed
        (bind _radius_off_on (Timeline|OFF/ON PlayFromStart)
          (:Update
            (Rendering|Lighting|SetAttenuationRadius _pointlight _radius_off_on)
            (Rendering|Components|Light|SetIntensity _pointlight_2 (Variables|Default|GetOnIntensity)))
          (:Finished
            (goto _label_2 Reset)))))
    (else
      (Utilities|FlowControl|DoOnce false :!label _label_2
        (:Completed
          (bind _off_on_intensity (Timeline|Timeline_0 PlayFromStart)
            (:Update
              (Rendering|Lighting|SetAttenuationRadius _pointlight _off_on_intensity)
              (Rendering|Components|Light|SetIntensity _pointlight_2 (Variables|Default|GetOffLightIntensity)))
            (:Finished
              (goto _label Reset))))))))

(event EventBeginPlay
  (Rendering|Lighting|SetAttenuationRadius (Variables|Default|GetPointLight) (Variables|Default|GetOffLightRadius))
  (Rendering|Components|Light|SetIntensity (Variables|Default|GetPointLight) (Variables|Default|GetOffLightIntensity)))

(fn ConstructionScript)